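; Enemy actor Blueprint that stays alive for a random lifetime of a few seconds.
; BeginPlay sets the alive flag and rolls the lifetime, which Tick counts down until it runs out and clears the flag.
; While counting down, Tick keeps the capsule component hidden in game, then unhides it on expiry without propagating to children.
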(event `self.ReceiveBeginPlay`
  (set `self.isAlive` true)
  (set `self.TimeLeft` (`KismetMathLibrary.RandomFloatInRange` 3.0 5.0)))

(event `self.ReceiveTick`
  (params (DeltaSeconds :type "Float (single-precision)"))
  (if (`self.isAlive`)
    (bind _output_get (set `self.TimeLeft` (- (`self.TimeLeft`) DeltaSeconds)))
    (bind _output_get_2 (set `self.isAlive` (> _output_get 0.0)))
    (`SceneComponent.SetHiddenInGame` (`self.CapsuleComponent`) _output_get_2 false)))

(fn `UserConstructionScript`)