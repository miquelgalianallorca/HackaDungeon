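; AI controller for the Minotaur enemy that chases the player and flags when it attacks.
; A looping one-second timer re-issues a move toward the player pawn unless the Minotaur's IsStunt flag is set.
; Each move request clears IsAttacking on the character, and a successful arrival sets it again unless the Minotaur is dead.
; The punch print and attack montage nodes are left unconnected.
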(event `self.ReceiveBeginPlay`
  (`KismetSystemLibrary.K2_SetTimer` null "FollowPlayer" 1.0 true))

(event `FollowPlayer`
  (bind _returnvalue (`self.K2_GetPawn`))
  (bind _asminotaur_character (cast `/Game/ThirdPersonBP/Characters/MinotaurCharacter` _returnvalue))
  (if (not (`/Game/ThirdPersonBP/Characters/MinotaurCharacter.isStunt` _asminotaur_character))
    (`|AIMoveTo` _returnvalue (0.0 0.0 0.0) (`GameplayStatics.GetPlayerPawn` 0)
      (:`then`
        (bind _asminotaur_character_2 (cast `/Game/ThirdPersonBP/Characters/MinotaurCharacter` _returnvalue))
        (set `/Game/ThirdPersonBP/Characters/MinotaurCharacter.isAttacking` false _asminotaur_character_2))
      (:`OnSuccess`
        (bind _asminotaur_character_3 (cast `/Game/ThirdPersonBP/Characters/MinotaurCharacter` _returnvalue))
        (if (not (`/Game/ThirdPersonBP/Characters/MinotaurCharacter.isDead` _asminotaur_character_3))
          (set `/Game/ThirdPersonBP/Characters/MinotaurCharacter.isAttacking` true _asminotaur_character_3))))))

(fn `UserConstructionScript`)