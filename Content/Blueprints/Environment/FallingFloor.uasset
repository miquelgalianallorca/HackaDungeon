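; A falling floor Blueprint that drops after a player steps on it.
; Overlap by a player-controlled pawn waits a configurable delay, then enables physics simulation on the box collision and flags it as falling.
; Hitting a component tagged "Floor" spawns a steam effect at the actor's transform and destroys the actor.
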(event `self.ReceiveActorBeginOverlap`
  (params (OtherActor :type "Actor Object Reference"))
  (bind _aspawn (cast `Pawn` OtherActor))
  (if (`Pawn.IsPlayerControlled` _aspawn)
    (`KismetSystemLibrary.Delay` (`self.delayToFall`))
    (`PrimitiveComponent.SetSimulatePhysics` (`self.BoxCollision`) true)
    (set `self.isFalling` true)))

(event `self.ReceiveHit`
  (params (MyComp :type "PrimitiveComponent Object Reference") (Other :type "Actor Object Reference") (OtherComp :type "PrimitiveComponent Object Reference") (bSelfMoved :type Boolean) (HitLocation :type "Vector Structure") (HitNormal :type "Vector Structure") (NormalImpulse :type "Vector Structure") (Hit :type "HitResult Structure (by ref)"))
  (if (`ActorComponent.ComponentHasTag` OtherComp "Floor")
    (`|SpawnActorFromClass` "/Game/Blueprints/Blueprint_Effect_Steam.Blueprint_Effect_Steam_C" (`self.GetTransform`) "Undefined" "OverrideRootScale" null null)
    (`self.K2_DestroyActor`)))

(fn `UserConstructionScript`)