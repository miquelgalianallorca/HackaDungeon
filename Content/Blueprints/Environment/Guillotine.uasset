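; Guillotine trap actor whose two blades endlessly slide shut and open, hurting player characters caught during the closing stroke.
; DoCut starts on BeginPlay and loops through close, pause, open and pause, using frame-length Delays and vector lerps instead of Tick or Timeline.
; The left blade mirrors the right on Y.
; Overlaps that begin while IsClosing launch the player's Character backward and up relative to the trap, then apply damage.
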(event `self.ReceiveBeginPlay`
  (`self.DoCut`))

(event `self.ReceiveActorBeginOverlap`
  (params (OtherActor :type "Actor Object Reference"))
  (bind _defaultsceneroot (`self.DefaultSceneRoot`))
  (bind _aspawn (cast `Pawn` OtherActor))
  (if (`Pawn.IsPlayerControlled` _aspawn)
    (if (`self.IsClosing`)
      (bind _ascharacter (cast `Character` _aspawn))
      (`Character.LaunchCharacter` _ascharacter (+ (* (`SceneComponent.GetForwardVector` _defaultsceneroot) -300.0) (* (`SceneComponent.GetUpVector` _defaultsceneroot) 200.0)) false false)
      (`GameplayStatics.ApplyDamage` OtherActor (`self.Damage`)))))

(event `DoCut`
  (bind _returnvalue (`GameplayStatics.GetWorldDeltaSeconds`))
  (bind _returnvalue_2 (`GameplayStatics.GetWorldDeltaSeconds`))
  (bind _timetemp (`self.TimeTemp`))
  (bind _closespeed (`self.CloseSpeed`))
  (bind _timetemp_2 (`self.TimeTemp`))
  (bind _openspeed (`self.OpenSpeed`))
  (set `self.TimeTemp` 0.0)
  (set `self.IsClosing` true :!label _label)
  (bind _returnvalue_3 (`KismetMathLibrary.VLerp` (`self.OpenedPosition`) (`self.ClosedPosition`) (`KismetMathLibrary.FClamp` (/ (stale _output_get_4) (`self.CloseSpeed`)))))
  (`SceneComponent.K2_SetRelativeLocation` (`self.SlashRight`) _returnvalue_3 false false)
  (`SceneComponent.K2_SetRelativeLocation` (`self.SlashLeft`) (`KismetMathLibrary.MakeVector` (.x _returnvalue_3) (* (.y _returnvalue_3) -1.0) (.z _returnvalue_3)) false false)
  (if (>= _timetemp _closespeed)
    (bind _output_get (set `self.TimeTemp` (- _timetemp _closespeed)))
    (set `self.IsClosing` false)
    (`KismetSystemLibrary.Delay` (- (`self.DelayClosed`) _output_get))
    (set `self.TimeTemp` 0.0)
    (bind _returnvalue_4 (`KismetMathLibrary.VLerp` (`self.ClosedPosition`) (`self.OpenedPosition`) (`KismetMathLibrary.FClamp` (/ (stale _output_get_3) (`self.OpenSpeed`)))))
    (`SceneComponent.K2_SetRelativeLocation` (`self.SlashRight`) _returnvalue_4 false false :!label _label_2)
    (`SceneComponent.K2_SetRelativeLocation` (`self.SlashLeft`) (`KismetMathLibrary.MakeVector` (.x _returnvalue_4) (* (.y _returnvalue_4) -1.0) (.z _returnvalue_4)) false false)
    (if (>= _timetemp_2 _openspeed)
      (bind _output_get_2 (set `self.TimeTemp` (- _timetemp_2 _openspeed)))
      (`KismetSystemLibrary.Delay` (- (`self.DelayOpened`) _output_get_2))
      (set `self.TimeTemp` 0.0)
      (else
        (`KismetSystemLibrary.Delay` _returnvalue_2)
        (bind _output_get_3 (set `self.TimeTemp` (+ (`self.TimeTemp`) _returnvalue_2)))
        (goto _label_2)))
    (else
      (`KismetSystemLibrary.Delay` _returnvalue)))
  (bind _output_get_4 (set `self.TimeTemp` (+ (`self.TimeTemp`) _returnvalue)))
  (goto _label))

(fn `UserConstructionScript`)