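; Spike hazard actor that damages and knocks away player-controlled characters that overlap it.
; On overlap it filters for a player-controlled Character, then launches it upward and backward relative to the spikes' root orientation, adding to its current velocity.
; It then applies damage to that character using the Damage variable.
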(event `self.ReceiveActorBeginOverlap`
  (params (OtherActor :type "Actor Object Reference"))
  (bind _defaultsceneroot (`self.DefaultSceneRoot`))
  (bind _aspawn (cast `Pawn` OtherActor))
  (if (`Pawn.IsPlayerControlled` _aspawn)
    (bind _ascharacter (cast `Character` _aspawn))
    (`Character.LaunchCharacter` _ascharacter (+ (* (`SceneComponent.GetForwardVector` _defaultsceneroot) -300.0) (* (`SceneComponent.GetUpVector` _defaultsceneroot) 1000.0)) false false)
    (`GameplayStatics.ApplyDamage` OtherActor (`self.Damage`))))

(fn `UserConstructionScript`)