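; FallingFloorSpawner is an environment actor that keeps a FallingFloor in place at its own transform.
; On BeginPlay it spawns the floor, passes it the fall delay and sets itself as the floor's spawner.
; Its RespawnFloor event waits a respawn delay and then loops back to the same spawn logic, replacing the current floor reference.
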(event `self.ReceiveBeginPlay`
  (bind _returnvalue (`|SpawnActorFromClass` "/Game/Blueprints/Environment/FallingFloor.FallingFloor_C" (`SceneComponent.K2_GetComponentToWorld` (`self.DefaultSceneRoot`)) "Undefined" "OverrideRootScale" null null :!label _label))
  (bind _output_get (set `self.CurrentFloor` _returnvalue))
  (set `/Game/Blueprints/Environment/FallingFloor.delayToFall` (`self.DelayToFall`) _output_get)
  (set `/Game/Blueprints/Environment/FallingFloor.MySpawner` self _output_get))

(event `RespawnFloor`
  (`KismetSystemLibrary.Delay` (`self.DelayToRespawn`))
  (goto _label))

(fn `UserConstructionScript`)