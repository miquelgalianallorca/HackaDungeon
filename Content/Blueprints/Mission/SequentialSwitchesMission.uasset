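; Mission Blueprint that checks whether a set of switches is being activated in array order.
; CheckMissionState walks the Switches array, flags the first inactive switch, and fails as soon as a later one is active.
; The state is valid whenever active switches form an unbroken run from the start, including none or all active.
; It only reads current Activated flags, with no event logic or stored press history.
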(fn `CheckMissionState`
  (returns (Accomplished :type Boolean))
  (set `self.SwitchIndex` 0)
  (set `self.FalseFound` false)
  (bind _output_get (set `self.ValidSequence` true))
  (while (and _output_get (< (`self.SwitchIndex`) (`KismetArrayLibrary.Array_Length` (`self.Switches`))))
    (if (`/Game/Blueprints/Mission/MissionSequentialSwitch.Activated` (`|GetArrayItem` (`self.Switches`) (`self.SwitchIndex`)))
      (if (`self.FalseFound`)
        (set `self.ValidSequence` false)
        (`/Engine/EditorBlueprintResources/StandardMacros.IncrementInt` (`self.SwitchIndex`) :!label _label))
      (else
        (set `self.FalseFound` true)
        (goto _label))))
  (return (`self.ValidSequence`)))