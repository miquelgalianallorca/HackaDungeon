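; Mission door that slides its static mesh down to open and back up to close.
; BeginPlay stores the closed position and an open position below it, scaled by the mesh's Z scale.
; OpenDoor and CloseDoor cancel each other and move the mesh through per-frame Delay loops instead of Tick or a Timeline.
; Each loop snaps to its target and updates Opened; the speed variables act as divisors, so larger values move slower.
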(event `self.ReceiveBeginPlay`
  (bind _staticmesh (`self.StaticMesh`))
  (bind (_returnvalue_x _returnvalue_y _returnvalue_z) (`KismetMathLibrary.BreakVector` (`SceneComponent.K2_GetComponentScale` _staticmesh)))
  (bind _output_get (set `self.ClosingTarget` (`SceneComponent.K2_GetComponentLocation` _staticmesh)))
  (set `self.OpeningTarget` (+ _output_get (`KismetMathLibrary.MakeVector` 0.0 0.0 (* -250.0 _returnvalue_z)))))

(event `OpenDoor`
  (bind _returnvalue (`KismetMathLibrary.MakeVector` 0.0 0.0 (* (/ 250.0 (`self.OpeningSpeed`)) (`self.DeltaSeconds`) -1.0)))
  (set `self.IsOpening` true)
  (if (`self.IsClosing`)
    (set `self.IsClosing` false))
  (if (`self.IsOpening`) :!label _label
    (set `self.DeltaSeconds` (`GameplayStatics.GetWorldDeltaSeconds`))
    (if (> (`KismetMathLibrary.VSizeSquared` _returnvalue) (`KismetMathLibrary.VSizeSquared` (- (`SceneComponent.K2_GetComponentLocation` (`self.StaticMesh`)) (`self.OpeningTarget`))))
      (`SceneComponent.K2_SetWorldLocation` (`self.StaticMesh`) (`self.OpeningTarget`) false false)
      (set `self.IsOpening` false)
      (set `self.Opened` true)
      (else
        (`SceneComponent.K2_AddLocalOffset` (`self.StaticMesh`) _returnvalue false false)
        (`KismetSystemLibrary.Delay` (`self.DeltaSeconds`))
        (goto _label)))))

(event `CloseDoor`
  (bind _returnvalue (`KismetMathLibrary.MakeVector` 0.0 0.0 (* (/ 250.0 (`self.ClosingSpeed`)) (`self.DeltaSeconds`))))
  (set `self.IsClosing` true)
  (if (`self.IsOpening`)
    (set `self.IsOpening` false))
  (if (`self.IsClosing`) :!label _label_2
    (set `self.DeltaSeconds` (`GameplayStatics.GetWorldDeltaSeconds`))
    (if (> (`KismetMathLibrary.VSizeSquared` _returnvalue) (`KismetMathLibrary.VSizeSquared` (- (`SceneComponent.K2_GetComponentLocation` (`self.StaticMesh`)) (`self.ClosingTarget`))))
      (`SceneComponent.K2_SetWorldLocation` (`self.StaticMesh`) (`self.ClosingTarget`) false false)
      (set `self.IsClosing` false)
      (set `self.Opened` false)
      (else
        (`SceneComponent.K2_AddLocalOffset` (`self.StaticMesh`) _returnvalue false false)
        (`KismetSystemLibrary.Delay` (`self.DeltaSeconds`))
        (goto _label_2)))))

(fn `UserConstructionScript`)