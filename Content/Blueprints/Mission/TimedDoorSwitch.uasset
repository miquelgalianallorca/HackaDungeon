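; TimedDoorSwitch is an overlap-triggered switch that opens a linked TimedDoor for a player-controlled pawn and closes it on a timer.
; It sets up a looping two-state switch at BeginPlay and calls ChangeState on both entering and leaving the overlap.
; Entering opens the door; leaving polls each frame through a Delay loop until the door reports Opened, then waits DelayToCloseDoor before closing it.
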(event `self.ReceiveBeginPlay`
  (`parent.ReceiveBeginPlay`)
  (set `self.LoopStates` true)
  (set `self.MaxState` 1)
  (set `self.CurrentState` 0))

(event `self.ReceiveActorBeginOverlap`
  (params (OtherActor :type "Actor Object Reference"))
  (bind _aspawn (cast `Pawn` OtherActor))
  (if (`Pawn.IsPlayerControlled` _aspawn)
    (`self.ChangeState`)
    (`/Game/Blueprints/Mission/Door.OpenDoor` (`self.TimedDoor`))))

(event `self.ReceiveActorEndOverlap`
  (params (OtherActor :type "Actor Object Reference"))
  (bind _timeddoor (`self.TimedDoor`))
  (bind _aspawn (cast `Pawn` OtherActor))
  (if (`Pawn.IsPlayerControlled` _aspawn)
    (`self.ChangeState`)
    (if (not (`/Game/Blueprints/Mission/Door.Opened` _timeddoor)) :!label _label
      (`KismetSystemLibrary.Delay` (`GameplayStatics.GetWorldDeltaSeconds`))
      (goto _label)
      (else
        (`KismetSystemLibrary.Delay` (`self.DelayToCloseDoor`))
        (`/Game/Blueprints/Mission/Door.CloseDoor` _timeddoor)))))

(fn `UserConstructionScript`
  (`parent.UserConstructionScript`))