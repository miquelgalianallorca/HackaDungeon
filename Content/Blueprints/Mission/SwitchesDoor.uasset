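; Mission door that opens once its switches mission check passes, presumably when the linked switches match a required state sequence.
; On BeginPlay it runs the parent logic, then passes its Switches and StatesSequence to SwitchesMissionInterface.
; While closed, it polls CheckMissionStateMessage every Tick, then latches Opened and calls OpenDoor on the first success.
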(event `self.ReceiveBeginPlay`
  (bind _switchesmissioninterface (`self.SwitchesMissionInterface`))
  (`parent.ReceiveBeginPlay`)
  (set `/Game/Blueprints/Mission/SwitchesMission.Switches` (`self.Switches`) _switchesmissioninterface)
  (set `/Game/Blueprints/Mission/SwitchesMission.StatesSequence` (`self.StatesSequence`) _switchesmissioninterface))

(event `self.ReceiveTick`
  (params (DeltaSeconds :type "Float (single-precision)"))
  (if (not (`self.Opened`))
    (bind _accomplished (message `/Game/Blueprints/Mission/iMission.CheckMissionState` (`self.SwitchesMissionInterface`)))
    (if _accomplished
      (set `self.Opened` _accomplished)
      (`self.OpenDoor`))))

(fn `UserConstructionScript`)