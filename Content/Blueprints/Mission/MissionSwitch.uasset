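; MissionSwitch is a touch-activated switch actor that steps through numbered states, showing each one as a material on its static mesh.
; On BeginPlay it applies the first entry of the Materials array, and each overlap by a player-controlled pawn calls ChangeState.
; ChangeState increments CurrentState up to MaxState, then either wraps to zero when LoopStates is set or stays put, using the state as the material index.
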(event `self.ReceiveBeginPlay`
  (`PrimitiveComponent.SetMaterial` (`self.StaticMesh`) 0 (`|GetArrayItem` (`self.Materials`))))

(event `self.ReceiveActorBeginOverlap`
  (params (OtherActor :type "Actor Object Reference"))
  (bind _aspawn (cast `Pawn` OtherActor))
  (if (`Pawn.IsPlayerControlled` _aspawn)
    (`self.ChangeState`)))

(fn `ChangeState`
  (bind _currentstate (`self.CurrentState`))
  (if (>= (`self.CurrentState`) (`self.MaxState`))
    (if (`self.LoopStates`)
      (set `self.CurrentState` 0)
      (`PrimitiveComponent.SetMaterial` (`self.StaticMesh`) 0 (`|GetArrayItem` (`self.Materials`) _currentstate) :!label _label))
    (else
      (`/Engine/EditorBlueprintResources/StandardMacros.IncrementInt` _currentstate
        (:`  `
          (goto _label))))))

(fn `UserConstructionScript`)