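; DefeatEnemiesDoor is a door that opens once its defeat-enemies mission is complete.
; On BeginPlay it hands its Enemies to DefeatEnemiesMission, which owns the completion check.
; While closed, it polls CheckMissionState every Tick, then sets Opened and calls OpenDoor on the first success, so the door opens only once.
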(event `self.ReceiveBeginPlay`
  (set `/Game/Blueprints/Mission/DefeatEnemiesMission.Enemies` (`self.Enemies`) (`self.DefeatEnemiesMission`)))

(event `self.ReceiveTick`
  (params (DeltaSeconds :type "Float (single-precision)"))
  (if (not (`self.Opened`))
    (bind _accomplished (`/Game/Blueprints/Mission/iMission.CheckMissionState` (`self.DefeatEnemiesMission`)))
    (if _accomplished
      (set `self.Opened` _accomplished)
      (`self.OpenDoor`))))

(fn `UserConstructionScript`)