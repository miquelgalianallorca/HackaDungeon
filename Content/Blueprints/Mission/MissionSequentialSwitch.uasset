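; MissionSequentialSwitch is a mission switch actor that turns on when a player-controlled pawn overlaps it.
; The first such overlap sets an Activated flag and applies the second entry of its Materials array to mesh slot 1; later overlaps are ignored.
; ResetSwitch clears the flag and applies the first material, but to slot 0 rather than slot 1.
; Any sequence ordering is handled outside this Blueprint.
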(event `self.ReceiveActorBeginOverlap`
  (params (OtherActor :type "Actor Object Reference"))
  (bind _aspawn (cast `Pawn` OtherActor))
  (if (and (`Pawn.IsPlayerControlled` _aspawn) (not (`self.Activated`)))
    (set `self.Activated` true)
    (`PrimitiveComponent.SetMaterial` (`self.StaticMesh`) 1 (`|GetArrayItem` (`self.Materials`) 1))))

(fn `ResetSwitch`
  (set `self.Activated` false)
  (`PrimitiveComponent.SetMaterial` (`self.StaticMesh`) 0 (`|GetArrayItem` (`self.Materials`))))

(fn `UserConstructionScript`)